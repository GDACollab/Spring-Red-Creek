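; MainCharacter is the sprite-based character that walks to a position held by BP_Camera, the player-controlled pawn.
; On BeginPlay it caches the camera and seeds its current and last character positions with its own location.
; Each tick it issues a SimpleMoveToLocation toward the camera's CharacterPos through its controller.
; It also sets the sprite's relative rotation to the negated capsule rotation, so the sprite does not turn with movement.
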(event EventBeginPlay
  (bind _asbp_camera (Utilities|Casting|CastToBP_Camera (Game|GetPlayerCharacter 0)))
  (bind _output_get (Variables|Default|SetMainCamera _asbp_camera))
  (bind _output_get_2 (Variables|/Game/RedCreek/Blueprints/BP_Camera.BP_Camera_C|SetCharacterPos _output_get (Transformation|GetActorLocation)))
  (Variables|/Game/RedCreek/Blueprints/BP_Camera.BP_Camera_C|SetLastCharacterLocation _output_get _output_get_2))

(event EventTick
  (params (DeltaSeconds :type Float%20%28single-precision%29))
  (Transformation|SetRelativeRotation (Variables|Default|GetSprite) (Class|KismetMathLibrary|NegateRotator (Transformation|GetWorldRotation (Variables|Collision|GetCapsuleComponent))) false false)
  (AI|Navigation|SimpleMovetoLocation (Pawn|GetController) (Variables|/Game/RedCreek/Blueprints/BP_Camera.BP_Camera_C|GetCharacterPos (Variables|Default|GetMainCamera))))

(fn ConstructionScript)