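; Clickable transition marker that moves the main character and the player-controlled BP_Camera to another area by teleporting both to target actors.
; An interact event sets Clicked, and Tick waits until the box collision registers an overlap before teleporting.
; It then updates the camera's stored positions and changes its ortho width.
; Cursor hover shows a name message, and Tick swaps the cube and cone material while hovered or clicked.
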(event OnComponentBeginOverlap(BoxCollision)
  (params (OverlappedComponent :type Primitive%20Component%20Object%20Reference) (OtherActor :type Actor%20Object%20Reference) (OtherComp :type Primitive%20Component%20Object%20Reference) (OtherBodyIndex :type Integer) (bFromSweep :type Boolean) (SweepResult :type Hit%20Result%20Structure%20%28by%20ref%29))
  (Variables|Default|SetCharacter%20Overlap true))

(event OnComponentEndOverlap(BoxCollision)
  (params (OverlappedComponent :type Primitive%20Component%20Object%20Reference) (OtherActor :type Actor%20Object%20Reference) (OtherComp :type Primitive%20Component%20Object%20Reference) (OtherBodyIndex :type Integer))
  (Variables|Default|SetCharacter%20Overlap false))

(event Custom|Unclicked
  (Variables|Default|SetClicked false))

(event Custom|Highlight
  (if (or (Variables|Default|GetClicked) (Variables|Default|GetHovered%20Over))
    (Rendering|Material|SetMaterial (Variables|Default|GetCube) 0 "/Game/StarterAssets/Materials/HoverOverSceneTransitionMaterial.HoverOverSceneTransitionMaterial")
    (else
      (Rendering|Material|SetMaterial (Variables|Default|GetCube) 0 "/Game/StarterAssets/Materials/SceneTransitionMaterial.SceneTransitionMaterial"))))

(event Custom|OnInteractedWith
  (Variables|Default|SetClicked true))

(event MouseInput|EventActorBeginCursorOver
  (Class|BPIMouse|OnHover(Message) (Game|GetPlayerCharacter 0) (Variables|Default|GetName))
  (Variables|Default|SetHovered%20Over true))

(event MouseInput|EventActorEndCursorOver
  (Class|BPIMouse|OnRelease(Message) (Game|GetPlayerCharacter 0))
  (Variables|Default|SetHovered%20Over false))

(event EventTick
  (params (DeltaSeconds :type Float%20%28single-precision%29))
  (CallFunction|Highlight)
  (if (Variables|Default|GetClicked)
    (if (Variables|Default|GetCharacter%20Overlap)
      (Transformation|Teleport (Game|GetPlayerCharacter 0) (Transformation|GetActorLocation (Variables|Default|GetNew%20Camera%20Position)) "0, 0, 0")
      (Transformation|Teleport (Variables|Default|GetReference%20Main%20Character) (Transformation|GetActorLocation (Variables|Default|GetNew%20Character%20Position)) "0, 0, 0")
      (bind _asbp_camera (Utilities|Casting|CastToBP_Camera (Game|GetPlayerCharacter 0)))
      (Variables|/Game/RedCreek/Blueprints/BP_Camera.BP_Camera_C|SetCharacterPos _asbp_camera (Transformation|GetActorLocation (Variables|Default|GetNew%20Character%20Position)))
      (Variables|Default|SetClicked false)
      (bind _asbp_camera_2 (Utilities|Casting|CastToBP_Camera (Game|GetPlayerCharacter 0)))
      (Variables|/Game/RedCreek/Blueprints/BP_Camera.BP_Camera_C|SetLastCharacterLocation _asbp_camera_2 (Transformation|GetActorLocation (Variables|Default|GetNew%20Character%20Position)))
      (Variables|/Game/RedCreek/Blueprints/BP_Camera.BP_Camera_C|SetLastCameraLocation _asbp_camera_2 (Transformation|GetActorLocation (Variables|Default|GetNew%20Camera%20Position)))
      (Default|ChangeOrtho _asbp_camera_2 (Variables|Default|GetNew%20Ortho%20Width)))))

(event EventBeginPlay
  (EventDispatchers|BindEventtoInteract (delegate Custom|OnInteractedWith)))

(fn ConstructionScript
  (|CallParentFunction))