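; BP_Interactable is a point-and-click interactable actor, apparently a base for objects the player can hover over, use and observe.
; Cursor hover events tell the player character to show the object's Name, then release the message when the cursor leaves.
; Interface click events call CallInteract on left click and print the object's ObserveText on right click.
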(event MouseInput|EventActorBeginCursorOver
  (Class|BPIMouse|OnHover(Message) (Game|GetPlayerCharacter 0) (Variables|Default|GetName)))

(event MouseInput|EventActorEndCursorOver
  (Class|BPIMouse|OnRelease(Message) (Game|GetPlayerCharacter 0)))

(event EventBPIonRightClick
  (Development|PrintString (Variables|Default|GetObserveText)))

(event EventBPIonLeftClick
  (Default|CallInteract))

(fn ConstructionScript)