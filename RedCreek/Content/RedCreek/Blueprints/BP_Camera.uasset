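; BP_Camera is the player's point-and-click hub, handling cursor input, UI screens and inventory.
; BeginPlay enables the mouse cursor and creates the HUD, pause menu and inventory widgets, which pause and inventory inputs swap on screen.
; Clicks trace under the cursor and message actors through BPI_Mouse, with left-click hits also setting CharacterPos.
; Events update hover text, restore the HUD on unpause and add items to a size-limited inventory.
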(event Custom|UnPause
  ;[1 1 1] Pause
  (UserInterface|Viewport|AddtoViewport (Variables|Default|GetHUD) 0))

(event Custom|AddToInventory
  (params (ItemToAdd :type Struct%20Pick%20Up%20Info%20Structure))
  (if (<= (Utilities|Array|Length (Variables|Default|GetInventory)) 12)
    (Utilities|Array|Add (Variables|Default|GetInventory) ItemToAdd)))

(event EventBeginPlay
  (bind _returnvalue (Game|GetPlayerController 0))
  ;[1 0.1938 0.5935] Begin Play
  (Variables|/Script/Engine.PlayerController|SetbShowMouseCursor _returnvalue true)
  (Variables|/Script/Engine.PlayerController|SetbEnableMouseOverEvents _returnvalue true)
  (bind _returnvalue_2 (UserInterface|CreateWidget "/Game/RedCreek/Blueprints/UserInterface/UI.UI_C"))
  (bind _output_get (Variables|Default|SetHUD _returnvalue_2))
  (UserInterface|Viewport|AddtoViewport _output_get 0)
  (bind _returnvalue_3 (UserInterface|CreateWidget "/Game/RedCreek/Blueprints/UserInterface/PauseMenu.PauseMenu_C"))
  (Variables|Default|SetPauseMenu _returnvalue_3)
  (bind _returnvalue_4 (UserInterface|CreateWidget "/Game/RedCreek/Blueprints/UserInterface/InventoryPopUp.InventoryPopUp_C"))
  (Variables|Default|SetInventoryUI _returnvalue_4))

(event EventOnHover
  (params (DisplayText :type String))
  ;[1 1 1] Hover
  (Variables|Default|SetHoverText DisplayText))

(event EventOnRelease
  ;[1 1 1] Hover
  (Variables|Default|SetHoverText ""))

(event Input|ActionEvents|InputActionPause
  (params (Key :type Key%20Structure :default "AnyKey"))
  ;[1 1 1] Pause
  (:Pressed
    (Game|SetGamePaused true)
    (Widget|RemovefromParent (Variables|Default|GetHUD))
    (UserInterface|Viewport|AddtoViewport (Variables|Default|GetPauseMenu) 0)))

(event Input|ActionEvents|InputActionRightClick
  (params (Key :type Key%20Structure :default "AnyKey"))
  (bind _returnvalue (Game|GetPlayerController 0))
  (bind _hitresult (Game|Player|GetHitResultUnderCursorbyChannel _returnvalue "TraceTypeQuery1" true))
  (bind _hitactor (Collision|BreakHitResult _hitresult))
  ;[1 1 1] Left and Right Click
  (:Pressed
    (if (Utilities|DoesObjectImplementInterface _hitactor "/Game/RedCreek/Blueprints/BPI_Mouse.BPI_Mouse_C")
      (Class|BPIMouse|BPIonRightClick(Message) _hitactor))))

(event Input|ActionEvents|InputActionLeftClick
  (params (Key :type Key%20Structure :default "AnyKey"))
  (bind _returnvalue (Game|GetPlayerController 0))
  (bind _returnvalue_2 (Game|GetPlayerController 0))
  (bind _hitresult (Game|Player|GetHitResultUnderCursorbyChannel _returnvalue "TraceTypeQuery1" true))
  (bind (_hitresult_2 _returnvalue_3) (Game|Player|GetHitResultUnderCursorbyChannel _returnvalue_2 "TraceTypeQuery1" true))
  (bind _hitactor (Collision|BreakHitResult _hitresult))
  ;[1 1 1] Left and Right Click
  (:Pressed
    (if (Utilities|DoesObjectImplementInterface _hitactor "/Game/RedCreek/Blueprints/BPI_Mouse.BPI_Mouse_C")
      (Class|BPIMouse|BPIonLeftClick(Message) _hitactor))
    (if _returnvalue_3
      (Variables|Default|SetCharacterPos (.Location (Collision|BreakHitResult _hitresult_2))))))

(event Input|ActionEvents|InputActionToggleInventory
  (params (Key :type Key%20Structure :default "AnyKey"))
  ;[1 1 1] Toggle Inventory
  (:Pressed
    (Utilities|FlowControl|FlipFlop
      (:A
        (Widget|RemovefromParent (Variables|Default|GetHUD))
        (UserInterface|Viewport|AddtoViewport (Variables|Default|GetInventoryUI) 0))
      (:B
        (Widget|RemovefromParent (Variables|Default|GetInventoryUI))
        (UserInterface|Viewport|AddtoViewport (Variables|Default|GetHUD) 0)))))

(fn ConstructionScript)