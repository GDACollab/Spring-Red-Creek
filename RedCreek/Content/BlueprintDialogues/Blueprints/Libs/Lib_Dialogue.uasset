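; Blueprint dialogue helper library for looking up speaker attributes and dialogue items, resolving branch hosts, and evaluating item traits and conditions.
; Lookups and branch resolution go through interface-checked messages to the datatable host or response handler.
; A script interpreter expands variables in traits, which become a lowercase, trimmed, semicolon-split list.
; It also runs condition scripts with the branch host as custom handler, treating empty conditions as passing.
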(fn GetSpeakerAttributes
  (params (DatatableHost :type Object%20Object%20Reference) (SpeakerID :type Name :default "None"))
  (Utilities|FlowControl|Sequence
    (:then_0
      (if (Utilities|DoesObjectImplementInterface DatatableHost "/Game/BlueprintDialogues/Blueprints/Interfaces/BPI_DialogueDatatableHost.BPI_DialogueDatatableHost_C")
        (bind (_result _found) (Class|BPIDialogueDatatableHost|GetSpeakerAttributes(Message) DatatableHost SpeakerID))
        (if _found
          (LocalVariables|SetReturn%20Value _result)
          (LocalVariables|SetRecordFound true))))
    (:then_1
      (return (LocalVariables|GetReturn%20Value) (LocalVariables|GetRecordFound)))))

(fn GetDialogueItem
  (params (DatatableHost :type Object%20Object%20Reference) (RowName :type Name :default "None"))
  (Utilities|FlowControl|Sequence
    (:then_0
      (if (Utilities|DoesObjectImplementInterface DatatableHost "/Game/BlueprintDialogues/Blueprints/Interfaces/BPI_DialogueDatatableHost.BPI_DialogueDatatableHost_C")
        (bind (_item _found) (Class|BPIDialogueDatatableHost|GetDialogueItem(Message) DatatableHost RowName))
        (if _found
          (LocalVariables|SetResult _item))))
    (:then_1
      (return (LocalVariables|GetResult)))))

(fn ExtractDialogueBranchHost
  (params (RawBranch :type String) (Dialogue%20Response%20Handler :type Object%20Object%20Reference))
  (Utilities|FlowControl|Sequence
    (:then_0
      (if (Utilities|DoesObjectImplementInterface Dialogue%20Response%20Handler "/Game/BlueprintDialogues/Blueprints/Interfaces/BPI_DialogueResponseHandler.BPI_DialogueResponseHandler_C")
        (bind (_host _branch) (Class|BPIDialogueResponseHandler|ExtractDialogueBranchHost(Message) Dialogue%20Response%20Handler RawBranch))
        (LocalVariables|SetHostFound _host)
        (LocalVariables|SetBranchName _branch)))
    (:then_1
      (return (LocalVariables|GetHostFound) (LocalVariables|GetBranchName)))))

(fn ExtractDialogueTraits
  (params (Item :type Dialogue%20Table%20Item%20Structure) (ScriptInterpreter :type %20Object%20Reference))
  (Utilities|FlowControl|Sequence
    (:then_0
      (bind _result (Default|ParseStringforVariables ScriptInterpreter (.Traits (Utilities|Struct|BreakDialogue_TableItem Item)) false))
      (bind _output_get (LocalVariables|SetTraitsStringList (Utilities|String|ParseIntoArray (Utilities|String|ToLower _result) ";")))
      (for (_array_element _array_index) _output_get
        (Utilities|Array|SetArrayElem (LocalVariables|GetTraitsStringList) _array_index (Utilities|String|TrimTrailing (Utilities|String|Trim _array_element)))))
    (:then_1
      (return (LocalVariables|GetTraitsStringList)))))

(fn DialogueBranchMeetsConditions
  (params (Branch :type Name :default "None") (BranchHost :type Object%20Object%20Reference) (DialogueItem :type Dialogue%20Table%20Item%20Structure) (ScriptInterpreter :type %20Object%20Reference))
  (bind _conditions (Utilities|Struct|BreakDialogue_TableItem DialogueItem))
  (Utilities|FlowControl|Sequence
    (:then_0
      (if (> (Utilities|String|Len _conditions) 0)
        (bind _resolvedstring (Default|ExecuteScript ScriptInterpreter _conditions BranchHost))
        (bind _result (Default|BoolTest ScriptInterpreter _resolvedstring)) ; Note, any non-zero, non-false strings returns true
        (LocalVariables|SetSuccess _result)
        (else
          (LocalVariables|SetSuccess true))))
    (:then_1
      (return (LocalVariables|GetSuccess)))))